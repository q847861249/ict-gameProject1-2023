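; Opera house curtain actor that slides its SMSceneCurtain02 mesh sideways along world Y on demand.
; The custom events C_MoveRight and C_MoveLeft each restart their own timeline, moving the mesh toward positive and negative Y respectively.
; Each update lerps from the current location toward a small fixed offset using the Speed track, so travel accumulates per tick and depends on update count.
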(event EventBeginPlay)

(event Collision|EventActorBeginOverlap
  (params (OtherActor :type Actor%20Object%20Reference)))

(event EventTick
  (params (DeltaSeconds :type Float%20%28single-precision%29)))

(event Custom|C_MoveRight
  (bind _sm_scenecurtain02 (Variables|Default|GetSM_SceneCurtain02))
  (bind _returnvalue (Transformation|GetWorldLocation _sm_scenecurtain02))
  (bind _speed (Timeline|Timeline PlayFromStart)
    (:Update
      (Transformation|SetWorldLocation (Variables|Default|GetSM_SceneCurtain02) (Math|Vector|Lerp(Vector) (Transformation|GetWorldLocation (Variables|Default|GetSM_SceneCurtain02)) (Math|Vector|MakeVector (.x _returnvalue) (+ (.y _returnvalue) 8.0) (.z _returnvalue)) _speed) false false))))

(event Custom|C_MoveLeft
  (bind _sm_scenecurtain02 (Variables|Default|GetSM_SceneCurtain02))
  (bind _returnvalue (Transformation|GetWorldLocation _sm_scenecurtain02))
  (bind _speed (Timeline|Timeline_0 PlayFromStart)
    (:Update
      (Transformation|SetWorldLocation (Variables|Default|GetSM_SceneCurtain02) (Math|Vector|Lerp(Vector) (Transformation|GetWorldLocation (Variables|Default|GetSM_SceneCurtain02)) (Math|Vector|MakeVector (.x _returnvalue) (- (.y _returnvalue) 8.0) (.z _returnvalue)) _speed) false false))))

(fn ConstructionScript)