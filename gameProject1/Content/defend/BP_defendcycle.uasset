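; Shield actor for the EcoA76 player character's defense, built on a sphere with a dynamic material that dissolves in on spawn.
; Accepted hits briefly flash the edge color, set a hit position and animate a radius via timeline, and briefly block further hits.
; Each hit drains the player's Stamina, calling CGetup instead when damage meets or exceeds it.
; Close and destroy events animate DissolveAmount, then destroy the actor.
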(event Custom|close
  ;[1 1 1] Close sheild
  (bind _returnvalue (Rendering|Material|CreateDynamicMaterialInstance (Variables|Default|GetSphere) 0 (Rendering|Material|GetMaterial (Variables|Default|GetSphere) 0) "None" :!class /Script/Engine.PrimitiveComponent))
  (Variables|Default|SetM _returnvalue)
  (bind _newtrack_0 (Timeline|Timeline_0 PlayFromStart)
    (:Update
      (Rendering|Material|SetScalarParameterValue (Variables|Default|GetM) "DissolveAmount" _newtrack_0 :!class /Script/Engine.MaterialInstanceDynamic))
    (:Finished
      (Actor|DestroyActor))))

(event EventBeginPlay
  ;[1 1 1] Open Sheild
  (bind _returnvalue (Rendering|Material|CreateDynamicMaterialInstance (Variables|Default|GetSphere) 0 (Rendering|Material|GetMaterial (Variables|Default|GetSphere) 0) "None" :!class /Script/Engine.PrimitiveComponent))
  (Variables|Default|SetM _returnvalue)
  (bind _newtrack_0 (Timeline|Timeline Play)
    (:Update
      (Rendering|Material|SetScalarParameterValue (Variables|Default|GetM) "DissolveAmount" _newtrack_0 :!class /Script/Engine.MaterialInstanceDynamic))))

(event Custom|hit_react
  (params (damage :type Float%20%28double-precision%29) (forward :type Vector))
  ;[1 1 1] hit on sheild
  (Variables|Default|SetDamage damage)
  (if (and (Variables|Default|GetcanHit) (not (Variables|Default|GetisDisolveSheild)))
    (Variables|Default|SetcanHit false)
    (Utilities|FlowControl|Sequence
      (:then_0
        (Rendering|Material|SetVectorParameterValue (Variables|Default|GetM) "EdgeColor" (Utilities|Struct|MakeLinearColor 1e+02 0.0 0.0 1.0) :!class /Script/Engine.MaterialInstanceDynamic)
        (Utilities|FlowControl|Sequence
          (:then_0
            (Utilities|FlowControl|Delay 0.25)
            (Rendering|Material|SetVectorParameterValue (Variables|Default|GetM) "EdgeColor" (Utilities|Struct|MakeLinearColor 0.224215 0.869792 0.817818 0.0) :!class /Script/Engine.MaterialInstanceDynamic)
            (Variables|Default|SetcanHit true))
          (:then_1
            (CallFunction|FEcoA76ReduceStamina (Variables|Default|GetDamage)))))
      (:then_1
        (Rendering|Material|SetVectorParameterValue (Variables|Default|GetM) "pos" (Math|Conversions|ToLinearColor(Vector) forward) :!class /Script/Engine.MaterialInstanceDynamic)
        (bind _speed (Timeline|Timeline_2 PlayFromStart)
          (:Update
            (Rendering|Material|SetScalarParameterValue (Variables|Default|GetM) "radius" (* _speed 8e+01) :!class /Script/Engine.MaterialInstanceDynamic)))))))

(event Custom|D_destory
  (if (not (Variables|Default|GetisDisolveSheild))
    (Variables|Default|SetisDisolveSheild false)
    (bind _speed (Timeline|Timeline_1 Play)
      (:Update
        (Rendering|Material|SetScalarParameterValue (Variables|Default|GetM) "DissolveAmount" _speed :!class /Script/Engine.MaterialInstanceDynamic))
      (:Finished
        (Variables|Default|SetisDisolveSheild false)
        (Actor|DestroyActor)))))

(fn ConstructionScript)

(fn FEcoA76ReduceStamina
  (params (damage :type Float%20%28double-precision%29))
  ;[1 1 1] disolve when hit over stamina
  (LocalVariables|SetL_Damage damage)
  (bind _aseco_a76 (Utilities|Casting|CastToEcoA76 (Game|GetPlayerCharacter 0)))
  (Variables|Default|SetAs%20Eco%20A76 _aseco_a76)
  (if (<= (.stamina (Variables|/Game/EcoA76/Character/BluePrint/EcoA76.EcoA76_C|GetAttribute _aseco_a76)) (LocalVariables|GetL_Damage))
    (Default|CGetup (Variables|Default|GetAs%20Eco%20A76))
    (else
      (Default|FReduceStamina (Variables|Default|GetAs%20Eco%20A76) (LocalVariables|GetL_Damage)))))