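; Zombie mob Blueprint that supplies zombie-specific animations and a punch attack actor.
; On BeginPlay it fills the attack, directional hit-reaction and death animation variables, with left and right hits sharing one reaction, then calls the punch setup.
; The punch event spawns an AC_punch_zombie, stores it as Punch and snaps it to the mesh's "punch" socket.
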(event Custom|punch_on
  (bind _returnvalue (Game|SpawnActorfromClass "/Game/weaponActor/AC_punch_zombie.AC_punch_zombie_C" (Transformation|GetSocketTransform (Variables|Character|GetMesh) "punch" "RTS_Actor") "Undefined" 0 0))
  (bind _output_get (Variables|Default|Setpunch _returnvalue))
  (Transformation|AttachComponentToComponent _output_get (Variables|Character|GetMesh) "punch" "SnapToTarget" "SnapToTarget" "SnapToTarget" true))

(event EventBeginPlay
  (Variables|Default|SetAttackAnimattion (Utilities|Array|MakeArray "/Game/Zombie/ani/attack/attack_zombie.attack_zombie"))
  (Variables|Default|SetHitAnimationLeft "/Game/Zombie/ani/hit_react/Zombie_hit_react.Zombie_hit_react")
  (Variables|Default|SetHitAnimationRight "/Game/Zombie/ani/hit_react/Zombie_hit_react.Zombie_hit_react")
  (Variables|Default|SetHitAnimationMiddle "/Game/Zombie/ani/hit_react/Zombie_hi_react_large.Zombie_hi_react_large")
  (Variables|Default|SetDeadAnimation "/Game/Zombie/ani/dead/zombie_death_montage.zombie_death_montage")
  (CallFunction|Punchon))

(fn ConstructionScript)