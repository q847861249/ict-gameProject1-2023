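; Spawner actor for the SICKA mansion map that chains zombie spawns and opens a long door at the end.
; A custom event spawns a zombie at the actor's location, stores it and increments a spawn counter.
; Tick watches the stored zombie and respawns on each death until the counter hits five.
; After that death it opens the first AC_LongDoor found in the level.
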(event Custom|C_spawnZombie
  (bind _returnvalue (AI|SpawnAIFromClass "/Game/Zombie/bp_mobs_zombie.bp_mobs_zombie_C" 0 (Transformation|GetActorLocation) "0, 0, 0" false 0))
  (bind _asbp_mobs_zombie (Utilities|Casting|CastTobp_mobs_zombie _returnvalue))
  (Variables|Default|Setzombie _asbp_mobs_zombie)
  (Variables|Default|SettargetZombieAmount (+ (Variables|Default|GettargetZombieAmount) 1)))

(event EventTick
  (params (DeltaSeconds :type Float%20%28single-precision%29))
  (bind _zombie (Variables|Default|Getzombie))
  (Utilities|IsValid _zombie
    (:Is%20Valid
      (if (Variables|/Game/NPCcharacterBase/BP_NPCMobsBase.BP_NPCMobsBase_C|GetisDead _zombie)
        (if (== (Variables|Default|GettargetZombieAmount) 5)
          (bind _outactors (Actor|GetAllActorsOfClass "/Game/ThirdPersonBP/Blueprints/doorControl/AC_LongDoor.AC_LongDoor_C"))
          (Default|COpenDoor (Utilities|Array|Get(acopy) _outactors))
          (else
            (CallFunction|CSpawnZombie)))))))

(fn ConstructionScript)