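; Base Blueprint for a ranged mob NPC that shoots pawns it sees, takes hits and drops loot.
; PawnSensing drives it: sight stores an aim rotation and plays the shoot montage, while player noise triggers a timeline turn toward the player.
; Non-Tyrant hits spawn blood, pick a montage from hit normal Z, apply damage and show it in a widget.
; Death ignores pawn collision and spawns a random pickup at a downward trace.
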(event Custom|C_Attack
  (bind _arrow (Variables|Default|GetArrow))
  (if (and (not (Variables|check|Getis%20hitting)) (not (Variables|check|GetisAttack)))
    (Variables|check|SetisAttack true)
    (Animation|Montage|PlayMontage (Variables|Character|GetMesh) (Variables|needtoset|GetAnimation_shoot)
      (:OnCompleted
        _)
      (:OnInterrupted
        (Utilities|IsValid _arrow
          (:Is%20Valid
            (Actor|DestroyActor _arrow)))))
    (Variables|check|SetisAttack false)))

(event OnHearNoise(PawnSensing)
  (params (Instigator :type Pawn%20Object%20Reference) (Location :type Vector%20%28by%20ref%29 :default "0, 0, 0") (Volume :type Float%20%28single-precision%29))
  (if (Actor|ActorHasTag Instigator "Player")
    (if (not (Math|Boolean|ORBoolean (<= (.health (Variables|Default|GetAttribute)) 0.0) (Variables|check|Getis%20hitting) (Variables|check|GetisAttack)))
      (Utilities|FlowControl|Sequence
        (:then_0
          (Utilities|FlowControl|DoOnce false
            (:Completed
              (bind _aseco_a76 (Utilities|Casting|CastToEcoA76 (Game|GetPlayerCharacter 0)))
              (Variables|Default|SetAs%20Eco%20A76 _aseco_a76))))
        (:then_1
          (bind _newtrack_0 (Timeline|Timeline PlayFromStart)
            (:Update
              (Transformation|SetActorRotation (Math|Rotator|MakeRotator 0.0 0.0 (Math|Float|Lerp (.yaw (Transformation|GetActorRotation)) (.yaw (Math|Rotator|FindLookatRotation (Transformation|GetActorLocation) (Transformation|GetActorLocation (Variables|Default|GetAs%20Eco%20A76)))) _newtrack_0))))))))))

(event OnSeePawn(PawnSensing)
  (params (Pawn :type Pawn%20Object%20Reference))
  (CallFunction|CShoot (Math|Rotator|FindLookatRotation (Transformation|GetSocketLocation (Variables|Character|GetMesh) "spine") (Transformation|GetActorLocation Pawn))))

(event Custom|C_shoot
  (params (rotation :type Rotator))
  (Variables|Default|SetRotation rotation)
  (CallFunction|CAttack))

(event Custom|C_hitReaction
  (params (Noramal :type Vector) (damage :type Float%20%28double-precision%29) (H_EcoA76_location :type Vector))
  (Variables|Default|SetH%20Eco%20A76%20Location H_EcoA76_location)
  (Variables|Default|SetHit_normal Noramal)
  (Variables|Default|SetDamage damage)
  (if (and (not (Variables|check|GetisTyrant)) (not (Variables|check|Getis%20hitting)))
    (Niagara|SpawnSystematLocation "/Game/blood/FX_blood.FX_blood" (Transformation|GetActorLocation))
    (Variables|check|Setis%20hitting true)
    (if (> (.health (Variables|Default|GetAttribute)) 0.0)
      (bind _timedelay (CallFunction|FHitReaction))
      (if (Variables|check|GetCanRotation)
        (Variables|check|SetCanRotation false)
        (Transformation|SetActorRotation (Math|Rotator|MakeRotator 0.0 0.0 (.yaw (Math|Rotator|FindLookatRotation (Transformation|GetActorLocation) (Variables|Default|GetH%20Eco%20A76%20Location)))))
        (Utilities|FlowControl|Delay _timedelay)
        (Variables|check|SetCanRotation false)))))

(event EventTick
  (params (DeltaSeconds :type Float%20%28single-precision%29)))

(event Custom|C_deadReact
  (Variables|check|SetisDead true)
  (Collision|SetCollisionResponsetoChannel (Variables|Collision|GetCapsuleComponent) "ECC_Pawn" "ECR_Ignore")
  (Utilities|FlowControl|Sequence
    (:then_0
      (Animation|PlayAnimMontage (Variables|needtoset|GetDeadAnimation) 1.0 "None"))
    (:then_1
      (Utilities|FlowControl|DoOnce false
        (:Completed
          (CallFunction|FRandomItemDrop))))))

(fn ConstructionScript)

(fn FHitReaction
  (bind _hit_normal (Variables|Default|GetHit_normal))
  (if (> (.z _hit_normal) 0.0)
    (bind _returnvalue (Animation|PlayAnimMontage (Variables|needtoset|GetHit%20Animation%20Left) 1.0 "None"))
    (LocalVariables|SettimeForDelay _returnvalue)
    (elif (== (.z _hit_normal) 0.0)
      (bind _returnvalue_2 (Animation|PlayAnimMontage (Variables|needtoset|GetHit%20Animation%20Middle) 1.0 "None"))
      (LocalVariables|SettimeForDelay _returnvalue_2)
      (else
        (bind _returnvalue_3 (Animation|PlayAnimMontage (Variables|needtoset|GetHit%20Animation%20Right) 1.0 "None"))
        (LocalVariables|SettimeForDelay _returnvalue_3))))
  (CallFunction|FDamageCal (Variables|Default|GetDamage))
  (if (> (.health (Variables|Default|GetAttribute)) 0.0)
    (return (LocalVariables|GettimeForDelay))
    (else
      (CallFunction|CDeadReact))))

(fn FDamageCal
  (params (NewParam :type Float%20%28double-precision%29))
  (CallFunction|FDisplayDamageUI NewParam)
  (LocalVariables|Setdamage_ NewParam)
  (if (>= (- (.health (Variables|Default|GetAttribute)) (LocalVariables|Getdamage_)) 0.0)
    (Utilities|Struct|SetmembersinS_MobsBase (Variables|Default|GetAttribute) (- (.health (Variables|Default|GetAttribute)) (LocalVariables|Getdamage_)))
    (else
      (Utilities|Struct|SetmembersinS_MobsBase (Variables|Default|GetAttribute) 0.0)
      (Variables|check|SetisDead true))))

(fn FRandomItemDrop
  (bind _returnvalue (Transformation|GetActorLocation))
  (bind _outhit (Collision|LineTraceByChannel _returnvalue (- _returnvalue "0, 0,200.000000") "TraceTypeQuery1" false (Utilities|Array|MakeArray (Game|GetPlayerCharacter 0)) "None"))
  (Game|SpawnActorfromClass (Utilities|Select :Index (Math|Random|RandomIntegerinRange 0 8) :Option%200 "/Game/ThirdPersonBP/Blueprints/Gold_system/sliverGold.sliverGold_C" :Option%201 "/Game/ThirdPersonBP/Blueprints/Gold_system/Gold.Gold_C" :Option%202 "/Game/ThirdPersonBP/Blueprints/Gold_system/Gold2.Gold2_C" :Option%203 "/Game/ThirdPersonBP/Blueprints/Gold_system/Gold3.Gold3_C" :Option%204 "/Game/Bag/item/HP_Potion.HP_Potion_C" :Option%205 "/Game/Bag/item/MP_Potion.MP_Potion_C") (Math|Transform|MakeTransform (.Location (Collision|BreakHitResult _outhit)) (Math|Rotator|MakeRotator 0.0 0.0 0.0)) "AdjustIfPossibleButDontSpawnIfColliding" 0 0))

(fn FDisplayDamageUI
  (params (damage :type Float%20%28double-precision%29))
  (bind _returnvalue (UserInterface|CreateWidget "/Game/UI/PB_Damage.PB_Damage_C" 0 damage (.yaw (Transformation|GetActorRotation))))
  (UserInterface|SetWidget (Variables|Default|GetW_damage) _returnvalue))