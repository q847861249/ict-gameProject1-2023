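; Base NPC mob character that senses the player, fights, reacts to hits and dies.
; PawnSensing turns it toward noises and, on sight of the player, updates Distance to set speed and trigger random montage attacks.
; Non-Tyrant hits spawn blood, pick a montage by hit normal Z, apply damage and show it on a widget.
; Death ignores pawn collision, drops a random gold or potion pickup at the traced ground, then destroys the actor.
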(event EventBeginPlay)

(event Custom|C_hitReaction
  (params (Normal :type Vector) (Damage :type Float%20%28double-precision%29) (player_world_location :type Vector))
  (Variables|Hit|SetH_EcoA76_worldLocation player_world_location)
  (Variables|Hit|SetHit_normal Normal)
  (Variables|Hit|SetDamage Damage)
  (if (and (not (Variables|status|GetisTyrant)) (not (Variables|Status|Getis%20hitting)))
    (Utilities|FlowControl|Sequence
      (:then_0
        (Audio|PlaySoundatLocation "/Game/blood/blood_Cue.blood_Cue" "0, 0, 0" "0, 0, 0" 1.0 1.0 0.0 0 0 0 0))
      (:then_1
        (Niagara|SpawnSystematLocation "/Game/blood/FX_blood.FX_blood" (Transformation|GetActorLocation))
        (Variables|Status|Setis%20hitting true)
        (if (> (.health (Variables|Default|GetAttribute)) 0.0)
          (bind _timedelay (CallFunction|FHitReact))
          (if (Variables|Hit|GetCanRotation)
            (Variables|Hit|SetCanRotation false)
            (Transformation|SetActorRotation (Math|Rotator|MakeRotator 0.0 0.0 (.yaw (Math|Rotator|FindLookatRotation (Transformation|GetWorldLocation (Variables|Character|GetMesh)) (Variables|Hit|GetH_EcoA76_worldLocation)))))
            (Utilities|FlowControl|Delay _timedelay)
            (Variables|Hit|SetCanRotation true)))))))

(event Custom|C_Attack
  (bind _attackanimattion (Variables|needtoset|GetAttackAnimattion))
  (bind (_outitem _outindex) (Utilities|Array|Random _attackanimattion))
  (if (Math|Boolean|ANDBoolean (not (Variables|Attack|Getis%20Attacking)) (not (Variables|Status|GetisDead)) (not (Variables|Status|Getis%20hitting)) (<= (Variables|PawnSensing|Getdistance) (Variables|NeedToSet|Getattack_distance)))
    (Variables|Default|Setstate "NewEnumerator1")
    (Variables|PawnSensing|SetSpeed 0.0)
    (Variables|Attack|SetAttackIndex _outindex) ; use this value to control damage
    (Variables|Attack|Setis%20Attacking true)
    (Animation|Montage|PlayMontage (Variables|Character|GetMesh) _outitem (Variables|Attack|GetAttackPlayRate)
      (:OnCompleted
        _)
      (:OnInterrupted
        _))
    (Variables|Attack|Setis%20Attacking false)
    (Variables|Default|Setstate "NewEnumerator0")))

(event OnComponentHit(CapsuleComponent)
  (params (HitComponent :type Primitive%20Component%20Object%20Reference) (OtherActor :type Actor%20Object%20Reference) (OtherComp :type Primitive%20Component%20Object%20Reference) (NormalImpulse :type Vector :default "0, 0, 0") (Hit :type Hit%20Result%20Structure%20%28by%20ref%29))
  ;[1 1 1] hit on ecoa76
  (if (Actor|ActorHasTag OtherActor "Player")
    (Variables|PawnSensing|Setdistance 1.5e+02)
    (CallFunction|CAttack)))

(event OnSeePawn(PawnSensing)
  (params (Pawn :type Pawn%20Object%20Reference))
  ;[1 1 1] when character see player
  (if (and (Actor|ActorHasTag Pawn "Player") (not (Variables|Status|GetisDead)))
    (bind _aseco_a76 (Utilities|Casting|CastToEcoA76 (Game|GetPlayerCharacter 0)))
    (Variables|Components|SetEcoA76 _aseco_a76)
    (if (Variables|/Game/EcoA76/Character/BluePrint/EcoA76.EcoA76_C|GetisDead _aseco_a76)
      (Variables|PawnSensing|SetSpeed 0.0)
      (else
        (Variables|PawnSensing|SetEcoA76%20World%20Location (Transformation|GetWorldLocation (Variables|/Script/Engine.Character|GetMesh (Variables|Components|GetEcoA76))))
        (Variables|PawnSensing|Setdistance (Math|Vector|Distance(Vector) (Transformation|GetWorldLocation (Variables|/Script/Engine.Character|GetMesh (Variables|Components|GetEcoA76))) (Transformation|GetWorldLocation (Variables|Character|GetMesh))))
        (switch Utilities|FlowControl|Switch|SwitchonE_mobs (Variables|Default|Getstate)
          (:NewEnumerator0
            (CallFunction|CMoveForward)
            (CallFunction|CAttack)))))))

(event OnHearNoise(PawnSensing)
  (params (Instigator :type Pawn%20Object%20Reference) (Location :type Vector%20%28by%20ref%29 :default "0, 0, 0") (Volume :type Float%20%28single-precision%29))
  ;[1 1 1] when character hearing player noise(use for rotation)
  (if (and (not (Variables|Status|GetisDead)) (not (Variables|Attack|Getis%20Attacking)))
    (bind _newtrack_0 (Timeline|Timeline PlayFromStart)
      (:Update
        (Transformation|SetActorRotation (Math|Rotator|MakeRotator 0.0 0.0 (Math|Float|Lerp (.yaw (Transformation|GetActorRotation)) (.yaw (Math|Rotator|FindLookatRotation (Transformation|GetActorLocation) (Transformation|GetActorLocation Instigator))) _newtrack_0)))))
    (else
      (Timeline|Timeline Stop))))

(event Custom|C_MoveForward
  ;[1 1 1] move forward in different distance
  (Variables|Default|Setstate "NewEnumerator0")
  (if (> (Variables|PawnSensing|Getdistance) 5e+02)
    (Variables|PawnSensing|SetSpeed 2.5e+02)
    (else
      (Variables|PawnSensing|SetSpeed 3.5e+02))))

(event Custom|C_deadReat
  (Variables|Status|SetisDead true)
  (Collision|SetCollisionResponsetoChannel (Variables|Collision|GetCapsuleComponent) "ECC_Pawn" "ECR_Ignore")
  (Utilities|FlowControl|Sequence
    (:then_0
      (Animation|PlayAnimMontage (Variables|NeedToSet|GetDeadAnimation) 1.0 "None"))
    (:then_1
      (Utilities|FlowControl|DoOnce false
        (:Completed
          (CallFunction|FRandomItemDrop))))
    (:then_2
      (Utilities|FlowControl|Delay 1e+01)
      (Actor|DestroyActor))))

(fn ConstructionScript)

(fn FHitReact
  (bind _hit_normal (Variables|Hit|GetHit_normal))
  (if (> (.z _hit_normal) 0.0)
    (bind _returnvalue (Animation|PlayAnimMontage (Variables|NeedToSet|GetHitAnimationRight) 1.0 "None"))
    (LocalVariables|SettimeForDelay _returnvalue)
    (elif (== (.z _hit_normal) 0.0)
      (bind _returnvalue_2 (Animation|PlayAnimMontage (Variables|NeedToSet|GetHitAnimationMiddle) 1.0 "None"))
      (LocalVariables|SettimeForDelay _returnvalue_2)
      (else
        (bind _returnvalue_3 (Animation|PlayAnimMontage (Variables|NeedToSet|GetHitAnimationLeft) 1.0 "None"))
        (LocalVariables|SettimeForDelay _returnvalue_3))))
  (CallFunction|FDamageCal (Variables|Hit|GetDamage))
  (if (> (.health (Variables|Default|GetAttribute)) 0.0)
    (return (LocalVariables|GettimeForDelay))
    (else
      (CallFunction|CDeadReat))))

(fn FDamageCal
  (params (Damage :type Float%20%28double-precision%29))
  (CallFunction|FDisplayDamageHit Damage)
  (LocalVariables|Setdamage_ Damage)
  (if (>= (- (.health (Variables|Default|GetAttribute)) (LocalVariables|Getdamage_)) 0.0)
    (Utilities|Struct|SetmembersinS_MobsBase (Variables|Default|GetAttribute) (- (.health (Variables|Default|GetAttribute)) (LocalVariables|Getdamage_)))
    (else
      (Utilities|Struct|SetmembersinS_MobsBase (Variables|Default|GetAttribute) 0.0)
      (Variables|Status|SetisDead true))))

(fn FRandomItemDrop
  (bind _returnvalue (Transformation|GetActorLocation))
  (bind _outhit (Collision|LineTraceByChannel _returnvalue (- _returnvalue "0, 0,200.000000") "TraceTypeQuery1" false (Utilities|Array|MakeArray (Game|GetPlayerCharacter 0)) "None"))
  (Game|SpawnActorfromClass (Utilities|Select :Index (Math|Random|RandomIntegerinRange 0 8) :Option%200 "/Game/ThirdPersonBP/Blueprints/Gold_system/sliverGold.sliverGold_C" :Option%201 "/Game/ThirdPersonBP/Blueprints/Gold_system/Gold.Gold_C" :Option%202 "/Game/ThirdPersonBP/Blueprints/Gold_system/Gold2.Gold2_C" :Option%203 "/Game/ThirdPersonBP/Blueprints/Gold_system/Gold3.Gold3_C" :Option%204 "/Game/Bag/item/HP_Potion.HP_Potion_C" :Option%205 "/Game/Bag/item/MP_Potion.MP_Potion_C") (Math|Transform|MakeTransform (.Location (Collision|BreakHitResult _outhit)) (Math|Rotator|MakeRotator 0.0 0.0 0.0)) "AdjustIfPossibleButDontSpawnIfColliding" 0 0))

(fn FDisplayDamageHit
  (params (Damage :type Float%20%28double-precision%29))
  (bind _returnvalue (UserInterface|CreateWidget "/Game/UI/PB_Damage.PB_Damage_C" 0 Damage))
  (UserInterface|SetWidget (Variables|Default|GetWidget) _returnvalue))