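; AC_shootBase is a base projectile actor for shooting attacks by EcoA76 and its enemies.
; On shoot it detaches, sets ProjectileMovement velocity from speed and direction, deactivates its capsule and sets a lifespan for self-destruction.
; Separate hit events pass damage and capsule forward vector to target-specific reactions: Gideon, Zombie and Steel enemies, or EcoA76 and its DefendCyle.
; Most reactions feed a shared hit-effect call using the supplied particle system.
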(event Custom|C_shootActor
  (params (Speed :type Float%20%28double-precision%29) (Direction :type Vector))
  (Transformation|DetachFromActor "KeepWorld" "KeepWorld" "KeepWorld")
  (Variables|/Script/Engine.MovementComponent|SetVelocity (Variables|Default|GetProjectileMovement) (* Speed Direction))
  (CallFunction|FDestoryActor))

(event Custom|C_hitReact_EcoA76
  (params (actor :type Actor%20Object%20Reference) (particleSystem :type Particle%20System%20Object%20Reference))
  ;[1 1 1] hit on Ecoa76 for enemy to use
  (Variables|Default|SetP%20System particleSystem)
  (bind _output_get (Variables|Default|SetForwardVector (Math|Vector|GetForwardVector (Variables|Default|GetCapsule))))
  (Utilities|FlowControl|Sequence
    (:then_0
      (bind _aseco_a76 (CallFunction|ReactEcoA76 actor (Variables|Default|GetDamage) _output_get))
      (CallFunction|PlayHitProjectile _aseco_a76 (Variables|Default|GetP%20System)))
    (:then_1
      (CallFunction|ReactDefendCyle actor (Variables|Default|GetDamage) _output_get))))

(event Custom|C_hitReact_Enemy
  (params (actor :type Actor%20Object%20Reference) (particleSystem :type Particle%20System%20Object%20Reference))
  ;[1 1 1] hit on enemy for ecoa76 to use
  (Variables|Default|SetP%20System particleSystem)
  (Variables|Default|SetForwardVector (Math|Vector|GetForwardVector (Variables|Default|GetCapsule)))
  (Utilities|FlowControl|Sequence
    (:then_0
      (bind _asgideon (CallFunction|ReactGideon actor (Variables|Default|GetDamage) (Variables|Default|GetForwardVector)))
      (CallFunction|PlayHitProjectile _asgideon (Variables|Default|GetP%20System)))
    (:then_1
      (bind _asbp_mobs_zombie (CallFunction|ReactZombie actor (Variables|Default|GetDamage) (Variables|Default|GetForwardVector)))
      (CallFunction|PlayHitProjectile _asbp_mobs_zombie (Variables|Default|GetP%20System)))
    (:then_2
      (bind _asbp_steel (CallFunction|ReactSteel actor (Variables|Default|GetDamage) (Variables|Default|GetForwardVector)))
      (CallFunction|PlayHitProjectile _asbp_steel (Variables|Default|GetP%20System)))))

(fn ConstructionScript)

(fn FDestoryActor
  (Components|Activation|Deactivate (Variables|Default|GetCapsule))
  (Actor|SetLifeSpan (Variables|Default|GetIn%20Lifespan)))