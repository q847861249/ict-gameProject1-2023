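; Gold pickup actor that adds its gold amount to the player's EcoA76 character when collected.
; Overlapping its box with a Player-tagged actor caches the EcoA76 reference, enables input and opens a gate.
; The pickup input action passes through that gate to add TotalGold, play a sound at the pickup's location and destroy the actor.
; No end-overlap handling closes the gate or disables input.
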(event OnComponentBeginOverlap(Box)
  (params (OverlappedComponent :type Primitive%20Component%20Object%20Reference) (OtherActor :type Actor%20Object%20Reference) (OtherComp :type Primitive%20Component%20Object%20Reference) (OtherBodyIndex :type Integer) (bFromSweep :type Boolean) (SweepResult :type Hit%20Result%20Structure%20%28by%20ref%29))
  (if (Actor|ActorHasTag OtherActor "Player")
    (bind _aseco_a76 (Utilities|Casting|CastToEcoA76 OtherActor))
    (Input|EnableInput (Game|GetPlayerController 0))
    (Utilities|FlowControl|Gate true) ; enters at Open
  ))

(event Custom|playSound
  (Audio|PlaySoundatLocation 0 (Transformation|GetActorLocation) "0, 0, 0" 1.0 1.0 0.0 0 0 0 0)
  (Actor|DestroyActor))

(event Input|EnhancedActionEvents|EnhancedInputActionIA_PickUP
  (params (ActionValue :type Boolean) (ElapsedSeconds :type Float%20%28double-precision%29) (TriggeredSeconds :type Float%20%28double-precision%29) (InputAction :type Input%20Action%20Object%20Reference :default "/Game/input/Action/IA_PickUP.IA_PickUP"))
  (:Triggered
    (Utilities|FlowControl|Gate true
      (:Exit
        (Default|FAddGold (stale OnComponentBeginOverlap(Box) _aseco_a76) (Variables|Default|GetTotal%20Gold))
        (CallFunction|PlaySound)))))

(fn ConstructionScript)