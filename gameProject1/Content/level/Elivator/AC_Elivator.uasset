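; Elevator actor that lowers its floor in two scripted stages, triggering level objects at each stop.
; C_down_2 and C_down_3 each use a timeline to lerp the floor down a fixed distance, the second continuing from the first's target height.
; The first stop opens all opera doors and switches on one opera light.
; The second sets the first big left travel door found to open.
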(event Custom|C_down_2
  (bind _floor (Variables|Default|Getfloor))
  (bind _returnvalue (Transformation|GetWorldLocation _floor))
  (Variables|Default|SetorginZ (.z (Transformation|GetWorldLocation (Variables|Default|Getfloor))))
  (Variables|Default|SetTagetDown (- (.z _returnvalue) 1.15e+03))
  (bind _newtrack_0 (Timeline|Timeline PlayFromStart)
    (:Update
      (Transformation|SetWorldLocation (Variables|Default|Getfloor) (Math|Vector|MakeVector (.x _returnvalue) (.y _returnvalue) (Math|Float|Lerp (Variables|Default|GetorginZ) (Variables|Default|GetTagetDown) _newtrack_0)) false false))
    (:Finished
      (Utilities|FlowControl|Sequence
        (:then_0
          (bind _outactors (Actor|GetAllActorsOfClass "/Game/level/Elivator/AC_operaDoor.AC_operaDoor_C"))
          (for _array_element _outactors
            (Default|COpen _array_element)))
        (:then_1
          (bind _outactors_2 (Actor|GetAllActorsOfClass "/Game/OperaHouse/Blueprints/AC_OperaLight.AC_OperaLight_C"))
          (Default|CSwitchonLight (Utilities|Array|Get(acopy) _outactors_2 1)))))))

(event Custom|C_down_3
  (bind _floor (Variables|Default|Getfloor))
  (bind _returnvalue (Transformation|GetWorldLocation _floor))
  (Variables|Default|SetorginZ (Variables|Default|GetTagetDown))
  (Variables|Default|SetTagetDown (- (Variables|Default|GetorginZ) 1.2e+03))
  (bind _newtrack_0 (Timeline|Timeline_0 PlayFromStart)
    (:Update
      (Transformation|SetWorldLocation (Variables|Default|Getfloor) (Math|Vector|MakeVector (.x _returnvalue) (.y _returnvalue) (Math|Float|Lerp (Variables|Default|GetorginZ) (Variables|Default|GetTagetDown) _newtrack_0)) false false))
    (:Finished
      (bind _outactors (Actor|GetAllActorsOfClass "/Game/BigStarStation/Maps/door/AC_TravelDoor_big_L.AC_TravelDoor_big_L_C"))
      (Variables|/Game/level/switchLevel/AC_GateBase.AC_GateBase_C|Setopen (Utilities|Array|Get(acopy) _outactors) true))))

(event EventBeginPlay)

(event Collision|EventActorBeginOverlap
  (params (OtherActor :type Actor%20Object%20Reference)))

(event EventTick
  (params (DeltaSeconds :type Float%20%28single-precision%29)))

(fn ConstructionScript)