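; Big double travel door actor that swings open when the player reaches it and then flags that travel is available.
; Overlap of TravelBox by a Player-tagged actor, while Open is true, plays a one-time sound and starts a Timeline.
; The Timeline lerps the yaw of leaves L and R in opposite directions from rotations cached on BeginPlay.
; On finish it sets CanTravel and activates the Niagara effect.
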(event OnComponentBeginOverlap(TravelBox)
  (params (OverlappedComponent :type Primitive%20Component%20Object%20Reference) (OtherActor :type Actor%20Object%20Reference) (OtherComp :type Primitive%20Component%20Object%20Reference) (OtherBodyIndex :type Integer) (bFromSweep :type Boolean) (SweepResult :type Hit%20Result%20Structure%20%28by%20ref%29))
  (bind _r (Variables|Default|GetR))
  (bind _l (Variables|Default|GetL))
  (bind _returnvalue (Transformation|GetWorldRotation _r))
  (bind _returnvalue_2 (Transformation|GetWorldRotation _l))
  (if (Variables|Default|Getopen)
    (if (Actor|ActorHasTag OtherActor "Player")
      (Utilities|FlowControl|Sequence
        (:then_0
          (Utilities|FlowControl|DoOnce false
            (:Completed
              (Audio|PlaySoundatLocation "/Game/AUDIO/door/door_open2.door_open2" (Transformation|GetActorLocation) "0, 0, 0" 1.0 1.0 0.0 0 0 0 0))))
        (:then_1
          (bind _newtrack_0 (Timeline|Timeline Play)
            (:Update
              (Utilities|FlowControl|Sequence
                (:then_0
                  (Transformation|SetWorldRotation (Variables|Default|GetL) (Math|Rotator|MakeRotator (.roll _returnvalue_2) (.pitch _returnvalue_2) (Math|Float|Lerp (Variables|Default|GetOriginY_L) (Variables|Default|GetTargetY_L) _newtrack_0)) false false))
                (:then_1
                  (Transformation|SetWorldRotation (Variables|Default|GetR) (Math|Rotator|MakeRotator (.roll _returnvalue) (.pitch _returnvalue) (Math|Float|Lerp (Variables|Default|GetOriginY_R) (Variables|Default|GetTargetY_R) _newtrack_0)) false false))))
            (:Finished
              (Variables|Default|SetcanTravel true)
              (Components|Activation|SetActive (Variables|Default|GetNiagara) true false))))))))

(event EventBeginPlay
  (bind _l (Variables|Default|GetL))
  (bind _r (Variables|Default|GetR))
  (bind _returnvalue (Transformation|GetWorldRotation _l))
  (bind _returnvalue_2 (Transformation|GetWorldRotation _r))
  (Variables|Default|SetOriginY_L (.yaw _returnvalue))
  (Variables|Default|SetTargetY_L (+ (.yaw _returnvalue) 85.0))
  (Variables|Default|SetOriginY_R (.yaw _returnvalue_2))
  (Variables|Default|SetTargetY_R (- (.yaw _returnvalue_2) 85.0)))

(fn ConstructionScript)