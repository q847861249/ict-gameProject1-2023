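; Gate base for switching levels, letting the player start travel by pressing interact at the gate.
; Player overlap on TravelBox enables input, and IA_Interact sets StartTravel if CanTravel is true, though this graph only ever clears that flag.
; While StartTravel is set, Tick repeatedly calls CStartTravel on EcoA76 with the level name and camera.
; Leaving the box clears both flags, calls CFinishTravel and disables input.
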(event OnComponentBeginOverlap(TravelBox)
  (params (OverlappedComponent :type Primitive%20Component%20Object%20Reference) (OtherActor :type Actor%20Object%20Reference) (OtherComp :type Primitive%20Component%20Object%20Reference) (OtherBodyIndex :type Integer) (bFromSweep :type Boolean) (SweepResult :type Hit%20Result%20Structure%20%28by%20ref%29))
  ;[1 1 1] Comment
  (if (Actor|ActorHasTag OtherActor "Player")
    (Input|EnableInput (Game|GetPlayerController 0))))

(event OnComponentEndOverlap(TravelBox)
  (params (OverlappedComponent :type Primitive%20Component%20Object%20Reference) (OtherActor :type Actor%20Object%20Reference) (OtherComp :type Primitive%20Component%20Object%20Reference) (OtherBodyIndex :type Integer))
  ;[1 1 1] afterOverLap
  (if (Actor|ActorHasTag OtherActor "Player")
    (Utilities|FlowControl|Sequence
      (:then_0
        (Variables|Default|SetcanTravel false))
      (:then_1
        (bind _aseco_a76 (Utilities|Casting|CastToEcoA76 OtherActor))
        (Default|CFinishTravel _aseco_a76))
      (:then_2
        (Variables|Default|SetstartTravel false)
        (Input|DisableInput (Game|GetPlayerController 0))))))

(event Input|EnhancedActionEvents|EnhancedInputActionIA_Interact
  (params (ActionValue :type Boolean) (ElapsedSeconds :type Float%20%28double-precision%29) (TriggeredSeconds :type Float%20%28double-precision%29) (InputAction :type Input%20Action%20Object%20Reference :default "/Game/input/Action/IA_Interact.IA_Interact"))
  ;[1 1 1] keyboard press event
  (:Triggered
    (if (and ActionValue (Variables|Default|GetcanTravel))
      (Variables|Default|SetstartTravel true))))

(event EventTick
  (params (DeltaSeconds :type Float%20%28single-precision%29))
  ;[1 1 1] Comment
  (if (Variables|Default|GetstartTravel)
    (bind _aseco_a76 (Utilities|Casting|CastToEcoA76 (stale OnComponentBeginOverlap(TravelBox) OtherActor)))
    (Default|CStartTravel _aseco_a76 (Variables|Default|GetlevelName) (Variables|Default|GetcameraRef))))

(fn ConstructionScript)