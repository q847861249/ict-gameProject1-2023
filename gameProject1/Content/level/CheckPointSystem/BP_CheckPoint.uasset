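; BP_CheckPoint is a one-shot checkpoint actor that saves its location when EcoA76 overlaps its sphere.
; UpdateSaveCheckPoint loads or creates the BP_SaveGame slot and writes the actor's location as the CheckPoint transform, with rotation and scale reset to defaults.
; It then shows a SavedGameNotification widget and destroys itself, so it cannot trigger again during that play session.
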(event OnComponentBeginOverlap(Sphere)
  (params (OverlappedComponent :type Primitive%20Component%20Object%20Reference) (OtherActor :type Actor%20Object%20Reference) (OtherComp :type Primitive%20Component%20Object%20Reference) (OtherBodyIndex :type Integer) (bFromSweep :type Boolean) (SweepResult :type Hit%20Result%20Structure%20%28by%20ref%29))
  (Utilities|Casting|CastToEcoA76 OtherActor)
  (|UpdateSaveCheckPoint)
  (bind _returnvalue (UserInterface|CreateWidget "/Game/level/CheckPointSystem/SavedGameNotification.SavedGameNotification_C"))
  (Default|DisplaySaveNotification _returnvalue)
  (UserInterface|Viewport|AddtoViewport _returnvalue 0)
  (Actor|DestroyActor))

(fn ConstructionScript)