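; Bedroom door actor that slides open along world X when an actor tagged Player enters its Box trigger, and slides back when that actor leaves.
; BeginPlay stores the mesh's starting X, and separate timelines drive opening and closing.
; Each update lerps from the current position, so opening accumulates small negative-X steps with no fixed end point, while closing eases toward the stored X.
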(event OnComponentBeginOverlap(Box)
  (params (OverlappedComponent :type Primitive%20Component%20Object%20Reference) (OtherActor :type Actor%20Object%20Reference) (OtherComp :type Primitive%20Component%20Object%20Reference) (OtherBodyIndex :type Integer) (bFromSweep :type Boolean) (SweepResult :type Hit%20Result%20Structure%20%28by%20ref%29))
  (bind _staticmesh (Variables|Default|GetStaticMesh))
  (bind _returnvalue (Transformation|GetWorldLocation _staticmesh))
  (if (Actor|ActorHasTag OtherActor "Player")
    (bind _newtrack_0 (Timeline|Timeline PlayFromStart)
      (:Update
        (Transformation|SetWorldLocation _staticmesh (Math|Vector|MakeVector (Math|Float|Lerp (.x _returnvalue) (- (.x _returnvalue) 2.0) _newtrack_0) (.y _returnvalue) (.z _returnvalue)) false false)))))

(event OnComponentEndOverlap(Box)
  (params (OverlappedComponent :type Primitive%20Component%20Object%20Reference) (OtherActor :type Actor%20Object%20Reference) (OtherComp :type Primitive%20Component%20Object%20Reference) (OtherBodyIndex :type Integer))
  (bind _staticmesh (Variables|Default|GetStaticMesh))
  (bind _returnvalue (Transformation|GetWorldLocation _staticmesh))
  (if (Actor|ActorHasTag OtherActor "Player")
    (bind _newtrack_0 (Timeline|Timeline_0 PlayFromStart)
      (:Update
        (Transformation|SetWorldLocation _staticmesh (Math|Vector|MakeVector (Math|Float|Lerp (.x _returnvalue) (Variables|Default|GetOriginX) _newtrack_0) (.y _returnvalue) (.z _returnvalue)) false false)))))

(event EventBeginPlay
  (Variables|Default|SetOriginX (.x (Transformation|GetWorldLocation (Variables|Default|GetStaticMesh)))))

(fn ConstructionScript)