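; Huge two-panel sliding door actor for the Big Star Station map, opened and closed through custom events with sound.
; BeginPlay caches each panel's closed world X and an asymmetric offset target, then snaps both to that open position.
; Open and close each run a timeline lerping L and R along world X, despite Y-named variables.
; Closing starts from the panels' current positions, while opening always starts from the cached closed ones.
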(event Custom|C_Close
  (bind _l (Variables|Default|GetL))
  (bind _r (Variables|Default|GetR))
  (bind _returnvalue (Transformation|GetWorldLocation _l))
  (bind _returnvalue_2 (Transformation|GetWorldLocation _r))
  (Variables|Default|SetCloseY_R (.x (Transformation|GetWorldLocation (Variables|Default|GetR))))
  (Variables|Default|SetCloseY_L (.x (Transformation|GetWorldLocation (Variables|Default|GetL))))
  (Audio|PlaySoundatLocation "/Game/AUDIO/door/Door_close.Door_close" (Transformation|GetActorLocation) "0, 0, 0" 1.0 1.0 0.0 0 0 0 0)
  (bind _newtrack_0 (Timeline|Timeline_0 PlayFromStart)
    (:Update
      (Utilities|FlowControl|Sequence
        (:then_0
          (Transformation|SetWorldLocation _l (Math|Vector|MakeVector (Math|Float|Lerp (Variables|Default|GetCloseY_L) (Variables|Default|GetOriginY_L) _newtrack_0) (.y _returnvalue) (.z _returnvalue)) false false))
        (:then_1
          (Transformation|SetWorldLocation _r (Math|Vector|MakeVector (Math|Float|Lerp (Variables|Default|GetCloseY_R) (Variables|Default|GetOriginY_R) _newtrack_0) (.y _returnvalue_2) (.z _returnvalue_2)) false false))))))

(event Custom|C_Open
  (bind _l (Variables|Default|GetL))
  (bind _r (Variables|Default|GetR))
  (bind _returnvalue (Transformation|GetWorldLocation _r))
  (bind _returnvalue_2 (Transformation|GetWorldLocation _l))
  (Audio|PlaySoundatLocation "/Game/AUDIO/door/door_open2.door_open2" (Transformation|GetActorLocation) "0, 0, 0" 1.0 1.0 0.0 0 0 0 0)
  (bind _newtrack_0 (Timeline|Timeline PlayFromStart)
    (:Update
      (Utilities|FlowControl|Sequence
        (:then_0
          (Transformation|SetWorldLocation (Variables|Default|GetL) (Math|Vector|MakeVector (Math|Float|Lerp (Variables|Default|GetOriginY_L) (Variables|Default|GetTargetY_L) _newtrack_0) (.y _returnvalue_2) (.z _returnvalue_2)) false false))
        (:then_1
          (Transformation|SetWorldLocation (Variables|Default|GetR) (Math|Vector|MakeVector (Math|Float|Lerp (Variables|Default|GetOriginY_R) (Variables|Default|GetTargetY_R) _newtrack_0) (.y _returnvalue) (.z _returnvalue)) false false))))))

(event Custom|C_setBeginLocation
  (bind _l (Variables|Default|GetL))
  (bind _r (Variables|Default|GetR))
  (bind _returnvalue (Transformation|GetWorldLocation _r))
  (bind _returnvalue_2 (Transformation|GetWorldLocation _l))
  (Transformation|SetWorldLocation _r (Math|Vector|MakeVector (Variables|Default|GetTargetY_R) (.y _returnvalue) (.z _returnvalue)) false false)
  (Transformation|SetWorldLocation _l (Math|Vector|MakeVector (Variables|Default|GetTargetY_L) (.y _returnvalue_2) (.z _returnvalue_2)) false false))

(event EventBeginPlay
  (bind _l (Variables|Default|GetL))
  (bind _r (Variables|Default|GetR))
  (bind _returnvalue (Transformation|GetWorldLocation _r))
  (bind _returnvalue_2 (Transformation|GetWorldLocation _l))
  (Variables|Default|SetOriginY_L (.x _returnvalue_2))
  (Variables|Default|SetTargetY_L (+ (.x _returnvalue_2) 4e+02))
  (Variables|Default|SetOriginY_R (.x _returnvalue))
  (Variables|Default|SetTargetY_R (- (.x _returnvalue) 2.5e+02))
  (CallFunction|CSetBeginLocation))

(fn ConstructionScript)