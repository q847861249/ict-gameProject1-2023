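; Small sliding travel door that opens for the player and marks travel as available once fully open.
; TravelBox overlaps by Player-tagged actors drive two timelines that lerp the mesh along world Y between its start and a fixed offset, with open and close sounds.
; Finishing the opening sets CanTravel and activates Niagara; leaving deactivates Niagara and closes from the current position, but never clears CanTravel.
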(event OnComponentBeginOverlap(TravelBox)
  (params (OverlappedComponent :type Primitive%20Component%20Object%20Reference) (OtherActor :type Actor%20Object%20Reference) (OtherComp :type Primitive%20Component%20Object%20Reference) (OtherBodyIndex :type Integer) (bFromSweep :type Boolean) (SweepResult :type Hit%20Result%20Structure%20%28by%20ref%29))
  (bind _worldlocation (Variables|Default|GetworldLocation))
  (if (Actor|ActorHasTag OtherActor "Player")
    (Audio|PlaySoundatLocation "/Game/AUDIO/door/door_open2.door_open2" (Transformation|GetActorLocation) "0, 0, 0" 1.0 1.0 0.0 0 0 0 0)
    (bind _newtrack_0 (Timeline|Timeline PlayFromStart)
      (:Update
        (Transformation|SetWorldLocation (Variables|Default|GetStaticMesh) (Math|Vector|MakeVector (.x _worldlocation) (Math|Float|Lerp (Variables|Default|GetOriginY) (Variables|Default|GetTargetY) _newtrack_0) (.z _worldlocation)) false false))
      (:Finished
        (Variables|Default|SetcanTravel true)
        (Components|Activation|SetActive (Variables|Default|GetNiagara) true false)))))

(event OnComponentEndOverlap(TravelBox)
  (params (OverlappedComponent :type Primitive%20Component%20Object%20Reference) (OtherActor :type Actor%20Object%20Reference) (OtherComp :type Primitive%20Component%20Object%20Reference) (OtherBodyIndex :type Integer))
  (bind _worldlocation (Variables|Default|GetworldLocation))
  (bind _worldlocation_2 (Variables|Default|GetworldLocation))
  (if (Actor|ActorHasTag OtherActor "Player")
    (Utilities|FlowControl|Sequence
      (:then_0
        (bind _newtrack_0 (Timeline|Timeline Stop)
          (:Update
            (Transformation|SetWorldLocation (Variables|Default|GetStaticMesh) (Math|Vector|MakeVector (.x _worldlocation_2) (Math|Float|Lerp (Variables|Default|GetOriginY) (Variables|Default|GetTargetY) _newtrack_0) (.z _worldlocation_2)) false false))
          (:Finished
            (Variables|Default|SetcanTravel true)
            (Components|Activation|SetActive (Variables|Default|GetNiagara) true false))))
      (:then_1
        (Variables|Default|SetcloseY (.y (Transformation|GetWorldLocation (Variables|Default|GetStaticMesh))))
        (Components|Activation|SetActive (Variables|Default|GetNiagara) false false)
        (Audio|PlaySoundatLocation "/Game/AUDIO/door/Door_close.Door_close" (Transformation|GetActorLocation) "0, 0, 0" 1.0 1.0 0.0 0 0 0 0)
        (bind _newtrack_0_2 (Timeline|Timeline_0 PlayFromStart)
          (:Update
            (Transformation|SetWorldLocation (Variables|Default|GetStaticMesh) (Math|Vector|MakeVector (.x _worldlocation) (Math|Float|Lerp (Variables|Default|GetcloseY) (Variables|Default|GetOriginY) _newtrack_0_2) (.z _worldlocation)) false false)))))))

(event EventBeginPlay
  (bind _staticmesh (Variables|Default|GetStaticMesh))
  (bind _returnvalue (Transformation|GetWorldLocation _staticmesh))
  (Variables|Default|SetworldLocation (Transformation|GetWorldLocation (Variables|Default|GetStaticMesh)))
  (Variables|Default|SetOriginY (.y _returnvalue))
  (Variables|Default|SetTargetY (- (.y _returnvalue) 1.4e+02)))

(fn ConstructionScript)