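; Large travel door actor for the BigStarStation map that slides its L and R panels apart along world Y when a Player-tagged actor enters TravelBox while Open is set.
; An opening timeline lerps the panels, then sets CanTravel and activates a Niagara effect.
; On exit it stops that timeline and a second one closes the panels from their current positions, switching the effect off; CanTravel is never cleared here.
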(event OnComponentBeginOverlap(TravelBox)
  (params (OverlappedComponent :type Primitive%20Component%20Object%20Reference) (OtherActor :type Actor%20Object%20Reference) (OtherComp :type Primitive%20Component%20Object%20Reference) (OtherBodyIndex :type Integer) (bFromSweep :type Boolean) (SweepResult :type Hit%20Result%20Structure%20%28by%20ref%29))
  (bind _r (Variables|Default|GetR))
  (bind _l (Variables|Default|GetL))
  (bind _returnvalue (Transformation|GetWorldLocation _l))
  (bind _returnvalue_2 (Transformation|GetWorldLocation _r))
  (if (Variables|Default|Getopen)
    (if (Actor|ActorHasTag OtherActor "Player")
      (Audio|PlaySoundatLocation "/Game/AUDIO/door/door_open2.door_open2" (Transformation|GetActorLocation) "0, 0, 0" 1.0 1.0 0.0 0 0 0 0)
      (bind _newtrack_0 (Timeline|Timeline PlayFromStart)
        (:Update
          (Utilities|FlowControl|Sequence
            (:then_0
              (Transformation|SetWorldLocation (Variables|Default|GetL) (Math|Vector|MakeVector (.x _returnvalue) (Math|Float|Lerp (Variables|Default|GetOriginY_L) (Variables|Default|GetTargetY_L) _newtrack_0) (.z _returnvalue)) false false))
            (:then_1
              (Transformation|SetWorldLocation (Variables|Default|GetR) (Math|Vector|MakeVector (.x _returnvalue_2) (Math|Float|Lerp (Variables|Default|GetOriginY_R) (Variables|Default|GetTargetY_R) _newtrack_0) (.z _returnvalue_2)) false false))))
        (:Finished
          (Variables|Default|SetcanTravel true)
          (Components|Activation|SetActive (Variables|Default|GetNiagara) true false))))))

(event OnComponentEndOverlap(TravelBox)
  (params (OverlappedComponent :type Primitive%20Component%20Object%20Reference) (OtherActor :type Actor%20Object%20Reference) (OtherComp :type Primitive%20Component%20Object%20Reference) (OtherBodyIndex :type Integer))
  (bind _r (Variables|Default|GetR))
  (bind _l (Variables|Default|GetL))
  (bind _l_2 (Variables|Default|GetL))
  (bind _r_2 (Variables|Default|GetR))
  (bind _returnvalue (Transformation|GetWorldLocation _l))
  (bind _returnvalue_2 (Transformation|GetWorldLocation _r))
  (bind _returnvalue_3 (Transformation|GetWorldLocation _l_2))
  (bind _returnvalue_4 (Transformation|GetWorldLocation _r_2))
  (if (Variables|Default|Getopen)
    (if (Actor|ActorHasTag OtherActor "Player")
      (Utilities|FlowControl|Sequence
        (:then_0
          (bind _newtrack_0 (Timeline|Timeline Stop)
            (:Update
              (Utilities|FlowControl|Sequence
                (:then_0
                  (Transformation|SetWorldLocation (Variables|Default|GetL) (Math|Vector|MakeVector (.x _returnvalue) (Math|Float|Lerp (Variables|Default|GetOriginY_L) (Variables|Default|GetTargetY_L) _newtrack_0) (.z _returnvalue)) false false))
                (:then_1
                  (Transformation|SetWorldLocation (Variables|Default|GetR) (Math|Vector|MakeVector (.x _returnvalue_2) (Math|Float|Lerp (Variables|Default|GetOriginY_R) (Variables|Default|GetTargetY_R) _newtrack_0) (.z _returnvalue_2)) false false))))
            (:Finished
              (Variables|Default|SetcanTravel true)
              (Components|Activation|SetActive (Variables|Default|GetNiagara) true false))))
        (:then_1
          (Variables|Default|SetCloseY_R (.y (Transformation|GetWorldLocation (Variables|Default|GetR))))
          (Variables|Default|SetCloseY_L (.y (Transformation|GetWorldLocation (Variables|Default|GetL))))
          (Components|Activation|SetActive (Variables|Default|GetNiagara) false false)
          (Audio|PlaySoundatLocation "/Game/AUDIO/door/Door_close.Door_close" (Transformation|GetActorLocation) "0, 0, 0" 1.0 1.0 0.0 0 0 0 0)
          (bind _newtrack_0_2 (Timeline|Timeline_0 PlayFromStart)
            (:Update
              (Utilities|FlowControl|Sequence
                (:then_0
                  (Transformation|SetWorldLocation _l_2 (Math|Vector|MakeVector (.x _returnvalue_3) (Math|Float|Lerp (Variables|Default|GetCloseY_L) (Variables|Default|GetOriginY_L) _newtrack_0_2) (.z _returnvalue_3)) false false))
                (:then_1
                  (Transformation|SetWorldLocation _r_2 (Math|Vector|MakeVector (.x _returnvalue_4) (Math|Float|Lerp (Variables|Default|GetCloseY_R) (Variables|Default|GetOriginY_R) _newtrack_0_2) (.z _returnvalue_4)) false false))))))))))

(event EventBeginPlay
  (bind _l (Variables|Default|GetL))
  (bind _r (Variables|Default|GetR))
  (bind _returnvalue (Transformation|GetWorldLocation _r))
  (bind _returnvalue_2 (Transformation|GetWorldLocation _l))
  (Variables|Default|SetOriginY_L (.y _returnvalue_2))
  (Variables|Default|SetTargetY_L (- (.y _returnvalue_2) 1.8e+02))
  (Variables|Default|SetOriginY_R (.y _returnvalue))
  (Variables|Default|SetTargetY_R (+ (.y _returnvalue) 1.9e+02)))

(fn ConstructionScript)