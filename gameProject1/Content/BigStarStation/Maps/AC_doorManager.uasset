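; Door manager actor for the BigStarStation map that sets travel doors open from progress flags on the PGI_LeveInstance game instance.
; On BeginPlay, the two boss flags (Steel, Revenant) each open one large travel door, and the BigmapDoor flag opens every small travel door.
; Large doors are picked by fixed index in GetAllActorsOfClass results, so the mapping depends on actor order.
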(event EventBeginPlay
  (bind _aspgi_leve_instance (Utilities|Casting|CastToPGI_LeveInstance (Game|GetGameInstance)))
  (Utilities|FlowControl|Sequence
    (:then_0
      (if (Variables|/Game/level/instance/PGI_LeveInstance.PGI_LeveInstance_C|GetcanOpenBossSteel _aspgi_leve_instance)
        (bind _outactors (Actor|GetAllActorsOfClass "/Game/BigStarStation/Maps/door/AC_TravelDoor_big_L.AC_TravelDoor_big_L_C"))
        (Variables|/Game/level/switchLevel/AC_GateBase.AC_GateBase_C|Setopen (Utilities|Array|Get(acopy) _outactors 1) true)))
    (:then_1
      (if (Variables|/Game/level/instance/PGI_LeveInstance.PGI_LeveInstance_C|GetcanOpenBossRevenant _aspgi_leve_instance)
        (bind _outactors_2 (Actor|GetAllActorsOfClass "/Game/BigStarStation/Maps/door/AC_TravelDoor_big_L.AC_TravelDoor_big_L_C"))
        (Variables|/Game/level/switchLevel/AC_GateBase.AC_GateBase_C|Setopen (Utilities|Array|Get(acopy) _outactors_2) true)))
    (:then_2
      (if (Variables|/Game/level/instance/PGI_LeveInstance.PGI_LeveInstance_C|GetbigmapDoor _aspgi_leve_instance)
        (bind _outactors_3 (Actor|GetAllActorsOfClass "/Game/BigStarStation/Maps/door/AC_TravelDoor_small.AC_TravelDoor_small_C"))
        (for _array_element _outactors_3
          (Variables|/Game/level/switchLevel/AC_GateBase.AC_GateBase_C|Setopen _array_element true))))))

(fn ConstructionScript)