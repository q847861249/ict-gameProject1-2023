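; BP_ch30 is an archer character that carries a bow and supplies its own shoot, hit and death animations.
; BeginPlay spawns the bow onto the mesh's "bow" socket and assigns the montages, with one front head-hit montage covering left, middle and right hits.
; A separate event spawns an arrow on the "arrow" socket and stores it in Arrow; nothing in this file calls it or fires the arrow.
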(event EventBeginPlay
  (CallFunction|CSpawnBow)
  (Variables|Default|SetAnimation_shoot "/Game/ch30/Animation/attack/Standing_Aim_Overdraw_binddummy_Anim_Montage.Standing_Aim_Overdraw_binddummy_Anim_Montage")
  (Variables|Default|SetHit%20Animation%20Left "/Game/ch30/Animation/hit/front_head_be_hit_Montage.front_head_be_hit_Montage")
  (Variables|Default|SetHit%20Animation%20Middle "/Game/ch30/Animation/hit/front_head_be_hit_Montage.front_head_be_hit_Montage")
  (Variables|Default|SetHit%20Animation%20Right "/Game/ch30/Animation/hit/front_head_be_hit_Montage.front_head_be_hit_Montage")
  (Variables|Default|SetDeadAnimation "/Game/ch30/Animation/dead/Standing_Death_Left_02_binddummy_Anim_Montage.Standing_Death_Left_02_binddummy_Anim_Montage"))

(event Custom|C_spawn%20bow
  (bind _returnvalue (Game|SpawnActorfromClass "/Game/weaponBase/AC_Bow.AC_Bow_C" (Transformation|GetSocketTransform (Variables|Character|GetMesh) "bow" "RTS_Actor") "Undefined" 0 0))
  (Transformation|AttachComponentToComponent _returnvalue (Variables|Character|GetMesh) "bow" "SnapToTarget" "SnapToTarget" "SnapToTarget" true))

(event Custom|C_spawn%20arrow
  (bind _returnvalue (Game|SpawnActorfromClass "/Game/ShootWeapon/arrow/AC_arrow.AC_arrow_C" (Transformation|GetSocketTransform (Variables|Character|GetMesh) "arrow" "RTS_Actor") "Undefined" 0 0))
  (bind _output_get (Variables|Default|SetArrow _returnvalue))
  (Transformation|AttachComponentToComponent _output_get (Variables|Character|GetMesh) "arrow" "SnapToTarget" "SnapToTarget" "SnapToTarget" true))

(fn ConstructionScript)