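; BP_PressureSwitchDoor is a door that a timeline slides vertically in response to pressure switch events.
; SwitchActivated and SwitchDeActivated raise or lower an active count, then play or reverse DoorOpen, which drives the door's relative Z.
; Both test PressureSwitches >= the active count, so while the count is within that limit, any activation opens the door and any deactivation closes it, without waiting for all switches.
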(event Custom|SwitchDeActivated
  (Math|Integer|DecrementInt (Variables|Default|GetPressureSwitchsActive)
    (:%20%20
      (if (>= (Variables|Default|GetPressureSwitches) (Variables|Default|GetPressureSwitchsActive))
        (bind _doorposition (Timeline|DoorOpen Reverse)
          (:Update
            (Transformation|SetRelativeLocation (Variables|Default|GetDoor) (Math|Vector|MakeVector 0.0 0.0 _doorposition) false false)))
        (else
          (Timeline|DoorOpen Play))))))

(event Custom|SwitchActivated
  (Math|Integer|IncrementInt (Variables|Default|GetPressureSwitchsActive)
    (:%20%20
      (if (>= (Variables|Default|GetPressureSwitches) (Variables|Default|GetPressureSwitchsActive))
        (bind _doorposition (Timeline|DoorOpen Play)
          (:Update
            (Transformation|SetRelativeLocation (Variables|Default|GetDoor) (Math|Vector|MakeVector 0.0 0.0 _doorposition) false false)))
        (else
          (Timeline|DoorOpen Reverse))))))

(event EventBeginPlay)

(event Collision|EventActorBeginOverlap
  (params (OtherActor :type Actor%20Object%20Reference)))

(event EventTick
  (params (DeltaSeconds :type Float%20%28single-precision%29)))

(fn ConstructionScript)