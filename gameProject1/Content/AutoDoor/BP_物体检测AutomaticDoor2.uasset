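; Automatic door that opens when a BP_PushableObject enters its Box trigger.
; The OpenDoor timeline lerps DoorL's relative Z to slide it open, with a sound played as it starts.
; End overlap is not filtered by class, so any actor leaving the box reverses the timeline, followed by a delayed close sound.
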(event OnComponentBeginOverlap(Box)
  (params (OverlappedComponent :type Primitive%20Component%20Object%20Reference) (OtherActor :type Actor%20Object%20Reference) (OtherComp :type Primitive%20Component%20Object%20Reference) (OtherBodyIndex :type Integer) (bFromSweep :type Boolean) (SweepResult :type Hit%20Result%20Structure%20%28by%20ref%29))
  (Utilities|Casting|CastToBP_PushableObject OtherActor)
  (CallFunction|DoorOpen))

(event OnComponentEndOverlap(Box)
  (params (OverlappedComponent :type Primitive%20Component%20Object%20Reference) (OtherActor :type Actor%20Object%20Reference) (OtherComp :type Primitive%20Component%20Object%20Reference) (OtherBodyIndex :type Integer))
  (CallFunction|DoorClose)
  (Utilities|FlowControl|Delay 1.0)
  (Audio|PlaySoundatLocation "/Game/AUDIO/door/Door_close.Door_close" (Transformation|GetActorLocation) "0, 0, 0" 1.0 1.0 0.0 0 0 0 0))

(event Custom|Door%20Open
  (Audio|PlaySoundatLocation "/Game/AUDIO/door/door_open2.door_open2" (Transformation|GetActorLocation) "0, 0, 0" 1.0 1.0 0.0 0 0 0 0)
  (bind _open (Timeline|OpenDoor Play)
    (:Update
      (Transformation|SetRelativeLocation (Variables|Default|GetDoor_L) (Math|Vector|MakeVector 0.0 0.0 (Math|Float|Lerp 1.2e+02 3.1e+02 _open)) false false))))

(event Custom|Door%20Close
  (bind _open (Timeline|OpenDoor Reverse)
    (:Update
      (Transformation|SetRelativeLocation (Variables|Default|GetDoor_L) (Math|Vector|MakeVector 0.0 0.0 (Math|Float|Lerp 1.2e+02 3.1e+02 _open)) false false))))

(event EventBeginPlay)

(event EventTick
  (params (DeltaSeconds :type Float%20%28single-precision%29)))

(fn ConstructionScript)