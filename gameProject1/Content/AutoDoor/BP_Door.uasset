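; BP_Door is an automatic sliding double door that opens when something enters its Box trigger and closes when it leaves.
; Box overlap events call DoorOpen and DoorClose, which play or reverse a single OpenDoor timeline.
; The timeline's Open track lerps the relative Y location of DoorL and DoorR, sliding the two panels apart in opposite directions.
; Overlaps are not filtered by actor or counted, so any end overlap starts closing the door.
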(event OnComponentBeginOverlap(Box)
  (params (OverlappedComponent :type Primitive%20Component%20Object%20Reference) (OtherActor :type Actor%20Object%20Reference) (OtherComp :type Primitive%20Component%20Object%20Reference) (OtherBodyIndex :type Integer) (bFromSweep :type Boolean) (SweepResult :type Hit%20Result%20Structure%20%28by%20ref%29))
  (CallFunction|DoorOpen))

(event OnComponentEndOverlap(Box)
  (params (OverlappedComponent :type Primitive%20Component%20Object%20Reference) (OtherActor :type Actor%20Object%20Reference) (OtherComp :type Primitive%20Component%20Object%20Reference) (OtherBodyIndex :type Integer))
  (CallFunction|DoorClose))

(event Custom|Door%20Open
  (bind _open (Timeline|OpenDoor Play)
    (:Update
      (Transformation|SetRelativeLocation (Variables|Default|GetDoor_L) (Math|Vector|MakeVector 0.0 (Math|Float|Lerp 1e+02 2e+02 _open) 0.0) false false)
      (Transformation|SetRelativeLocation (Variables|Default|GetDoor_R) (Math|Vector|MakeVector 0.0 (Math|Float|Lerp -1e+02 -2e+02 _open) 0.0) false false))))

(event Custom|Door%20Close
  (bind _open (Timeline|OpenDoor Reverse)
    (:Update
      (Transformation|SetRelativeLocation (Variables|Default|GetDoor_L) (Math|Vector|MakeVector 0.0 (Math|Float|Lerp 1e+02 2e+02 _open) 0.0) false false)
      (Transformation|SetRelativeLocation (Variables|Default|GetDoor_R) (Math|Vector|MakeVector 0.0 (Math|Float|Lerp -1e+02 -2e+02 _open) 0.0) false false))))

(event EventBeginPlay)

(event EventTick
  (params (DeltaSeconds :type Float%20%28single-precision%29)))

(fn ConstructionScript)