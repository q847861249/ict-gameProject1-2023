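; Climbable ladder actor that puts an EcoA76 character into and out of a climbing state.
; The construction script stacks a configurable count of ladder meshes at even spacing and applies transforms to the ladder and top collisions.
; Hold snaps the character in front of the ladder facing it at its current height, stops it, and sets Custom movement and IsClimbing.
; UnHold restores Walking and clears the flag; climbing motion is not handled here.
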(event EventBeginPlay)

(event Collision|EventActorBeginOverlap
  (params (OtherActor :type Actor%20Object%20Reference)))

(event EventTick
  (params (DeltaSeconds :type Float%20%28single-precision%29)))

(event EventHold
  (params (Character :type Character%20Object%20Reference))
  (CallFunction|HandleInteraction Character))

(event EventUnHold
  (params (Character :type Character%20Object%20Reference))
  (bind _aseco_a76 (Utilities|Casting|CastToEcoA76 Character))
  (bind _charactermovement (Variables|/Script/Engine.Character|GetCharacterMovement _aseco_a76))
  (Pawn|Components|CharacterMovement|SetMovementMode _charactermovement "MOVE_Walking" 0)
  (Variables|/Game/EcoA76/Character/BluePrint/EcoA76.EcoA76_C|SetIsClimbing _aseco_a76 false)
  (Variables|/Script/Engine.CharacterMovementComponent|SetbOrientRotationToMovement _charactermovement true))

(fn ConstructionScript
  (for _index (range 0 (- (Variables|Default|GetLadderCount) 1))
    (bind _returnvalue (AddComponent|AddStaticMeshComponent false (Math|Transform|MakeTransform (Math|Vector|MakeVector 0.0 0.0 (* _index (Variables|Default|GetDistanceBetweenLadder))) "0, 0, 0" "1.000000,1.000000,1.000000")))
    (Components|StaticMesh|SetStaticMesh _returnvalue (Variables|Default|GetLadderMesh)))
  (Transformation|SetRelativeTransform (Variables|Default|GetLadderCollision) (Variables|Default|GetLadderCollisionTransform) false false)
  (Transformation|SetRelativeTransform (Variables|Default|GetTopCollision) (Variables|Default|GetTopCollisionTransform) false false))

(fn HandleInteraction
  (params (Character :type Character%20Object%20Reference))
  (bind _returnvalue (Transformation|GetActorLocation))
  (bind _returnvalue_2 (Transformation|GetActorForwardVector))
  (bind _returnvalue_3 (Transformation|GetActorRotation))
  (bind _returnvalue_4 (* _returnvalue_2 4e+01))
  (bind _charactermovement (Variables|/Script/Engine.Character|GetCharacterMovement Character))
  (bind _returnvalue_5 (+ _returnvalue _returnvalue_4))
  (bind (_x _y) (Math|Vector|BreakVector _returnvalue_5))
  (Utilities|IsValid Character
    (:Is%20Valid
      (bind _output_get (Variables|Default|SetCharacterNewTransformLocation (Math|Transform|MakeTransform (Math|Vector|MakeVector _x _y (.Z (Math|Vector|BreakVector (Transformation|GetActorLocation Character)))) (Math|Rotator|MakeRotator (.roll _returnvalue_3) (.pitch _returnvalue_3) (+ (.yaw _returnvalue_3) 1.8e+02)) (.scale (Transformation|GetActorTransform Character)))))
      (Transformation|SetActorTransform Character _output_get true)
      (Pawn|Components|CharacterMovement|SetMovementMode _charactermovement "MOVE_Custom" 0)
      (Variables|/Game/EcoA76/Character/BluePrint/EcoA76.EcoA76_C|SetIsClimbing (.AsEco%20A76 (Utilities|Casting|CastToEcoA76 Character)) true)
      (Variables|/Script/Engine.CharacterMovementComponent|SetbOrientRotationToMovement _charactermovement true)
      (Components|Movement|StopMovementImmediately _charactermovement))))