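; Stage-change trigger actor that moves the game along when a Player-tagged actor passes through its Box.
; On BeginPlay it finds and stores BP_bgmcontrol, then calls BgmControl.
; Player overlap calls TeleportDragon on the first AC_stageend found.
; End overlap passes a DoOnce before the tag check, so only the first exiting actor counts; if it is the player, AC_spawngGideon spawns beside the Box and the trigger destroys itself.
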(event OnComponentBeginOverlap(Box)
  (params (OverlappedComponent :type Primitive%20Component%20Object%20Reference) (OtherActor :type Actor%20Object%20Reference) (OtherComp :type Primitive%20Component%20Object%20Reference) (OtherBodyIndex :type Integer) (bFromSweep :type Boolean) (SweepResult :type Hit%20Result%20Structure%20%28by%20ref%29))
  (if (Actor|ActorHasTag OtherActor "Player")
    (bind _outactors (Actor|GetAllActorsOfClass "/Game/Dragon/control/AC_stageend.AC_stageend_C"))
    (Default|TeleportDragon (Utilities|Array|Get(acopy) _outactors))))

(event OnComponentEndOverlap(Box)
  (params (OverlappedComponent :type Primitive%20Component%20Object%20Reference) (OtherActor :type Actor%20Object%20Reference) (OtherComp :type Primitive%20Component%20Object%20Reference) (OtherBodyIndex :type Integer))
  (bind _box (Variables|Default|GetBox))
  (bind _returnvalue (Transformation|GetWorldTransform _box))
  (Utilities|FlowControl|DoOnce false
    (:Completed
      (if (Actor|ActorHasTag OtherActor "Player")
        (Game|SpawnActorfromClass "/Game/Dragon/Attacker/AC_spawngGideon.AC_spawngGideon_C" (Math|Transform|MakeTransform (Math|Vector|MakeVector (+ (.x (.location _returnvalue)) 9e+01) (+ (.y (.location _returnvalue)) 2e+02) (.z (.location _returnvalue))) "0.000000,90.000000,0.000000" "1.000000,1.000000,1.000000") "Undefined" 0 0)
        (Actor|DestroyActor)))))

(event EventBeginPlay
  (bind _outactors (Actor|GetAllActorsOfClass "/Game/CASTELMAP/BP_bgmcontrol.BP_bgmcontrol_C"))
  (bind _output_get (Variables|Default|Setbgm (Utilities|Array|Get(acopy) _outactors)))
  (Default|BgmControl (Utilities|Array|Get(acopy) _outactors)))

(event Collision|EventActorBeginOverlap
  (params (OtherActor :type Actor%20Object%20Reference)))

(event EventTick
  (params (DeltaSeconds :type Float%20%28single-precision%29)))

(fn ConstructionScript)