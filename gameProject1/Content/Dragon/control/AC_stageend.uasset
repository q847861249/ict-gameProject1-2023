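; Stage actor that drives the flight cycle of the BP_flydragon boss or creature by repositioning it between marker boxes and arrows.
; Leaving the navigation box triggers falling, resets or a switch from Clean to Flyingup, depending on the dragon's state.
; Teleporting snaps the dragon to the side start or attack start and launches that state's behavior.
; Entering the attack end box turns Flyingup into Attack.
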(event OnComponentEndOverlap(box_navigation)
  (params (OverlappedComponent :type Primitive%20Component%20Object%20Reference) (OtherActor :type Actor%20Object%20Reference) (OtherComp :type Primitive%20Component%20Object%20Reference) (OtherBodyIndex :type Integer))
  (bind _dragon (Variables|Default|Getdragon))
  (switch Utilities|FlowControl|Switch|SwitchonE_Dragon (Variables|/Game/Dragon/BP_flydragon.BP_flydragon_C|GetState _dragon)
    (:NewEnumerator0
      (CallFunction|CFalling))
    (:NewEnumerator7
      (Variables|/Game/Dragon/BP_flydragon.BP_flydragon_C|Setspeed _dragon 0.0)
      (Variables|/Game/Dragon/BP_flydragon.BP_flydragon_C|SetState _dragon "NewEnumerator0")
      (CallFunction|TeleportDragon))
    (:NewEnumerator9
      (Default|FDestoryFire _dragon)
      (Utilities|FlowControl|Delay 2.0)
      (Variables|/Game/Dragon/BP_flydragon.BP_flydragon_C|Setenterclean _dragon false)
      (Variables|/Game/Dragon/BP_flydragon.BP_flydragon_C|Setspeed _dragon 0.0)
      (Variables|/Game/Dragon/BP_flydragon.BP_flydragon_C|SetState _dragon "NewEnumerator5")
      (CallFunction|TeleportDragon))))

(event OnComponentBeginOverlap(box_attack_end)
  (params (OverlappedComponent :type Primitive%20Component%20Object%20Reference) (OtherActor :type Actor%20Object%20Reference) (OtherComp :type Primitive%20Component%20Object%20Reference) (OtherBodyIndex :type Integer) (bFromSweep :type Boolean) (SweepResult :type Hit%20Result%20Structure%20%28by%20ref%29))
  (bind _dragon (Variables|Default|Getdragon))
  (switch Utilities|FlowControl|Switch|SwitchonE_Dragon (Variables|/Game/Dragon/BP_flydragon.BP_flydragon_C|GetState _dragon)
    (:NewEnumerator5
      (Variables|/Game/Dragon/BP_flydragon.BP_flydragon_C|SetFlying%20up _dragon false)
      (Variables|/Game/Dragon/BP_flydragon.BP_flydragon_C|SetState _dragon "NewEnumerator2")
      (Variables|/Game/Dragon/BP_flydragon.BP_flydragon_C|Setstart%20attack _dragon true))))

(event Custom|C_falling
  (bind _cool_down_clean (Variables|Default|GetCool%20Down%20Clean))
  (Default|CFalling (Variables|Default|Getdragon) _cool_down_clean)
  (Utilities|FlowControl|Delay (+ _cool_down_clean 5.0))
  (CallFunction|TeleportDragon))

(event Custom|teleport%20dragon
  (bind _outactors (Actor|GetAllActorsOfClass "/Game/Dragon/BP_flydragon.BP_flydragon_C"))
  (bind _output_get (Variables|Default|Setdragon (Utilities|Array|Get(acopy) _outactors)))
  (switch Utilities|FlowControl|Switch|SwitchonE_Dragon (Variables|/Game/Dragon/BP_flydragon.BP_flydragon_C|GetState _output_get)
    (:NewEnumerator0
      (CallFunction|CLocomotion))
    (:NewEnumerator5
      (CallFunction|CFlyingUp))
    (:NewEnumerator9
      (CallFunction|CClean))))

(event Custom|C_Locomotion
  (Transformation|SetActorRotation (Variables|Default|Getdragon) (Transformation|GetWorldRotation (Variables|Default|GetArrowSide)))
  (Transformation|SetActorLocation (Variables|Default|Getdragon) (Transformation|GetWorldLocation (Variables|Default|Getbox_start)) false false)
  (Default|MovetoEnd (Variables|Default|Getdragon)))

(event Custom|C_clean
  (Transformation|SetActorRotation (Variables|Default|Getdragon) (Transformation|GetWorldRotation (Variables|Default|GetArrowSide)))
  (Transformation|SetActorLocation (Variables|Default|Getdragon) (Transformation|GetWorldLocation (Variables|Default|Getbox_start)) false false)
  (Default|Clean (Variables|Default|Getdragon)))

(event Custom|C_flyingUp
  (Transformation|SetActorRotation (Variables|Default|Getdragon) (Transformation|GetWorldRotation (Variables|Default|GetArrowFront)))
  (Transformation|SetActorLocation (Variables|Default|Getdragon) (Transformation|GetWorldLocation (Variables|Default|Getbox_attack_start)) false false)
  (Variables|/Game/Dragon/BP_flydragon.BP_flydragon_C|SetFlying%20up (Variables|Default|Getdragon) true))

(event Custom|C_destoryend
  (Actor|DestroyActor))

(fn ConstructionScript)