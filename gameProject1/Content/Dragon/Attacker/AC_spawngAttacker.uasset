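; Spawner actor that keeps one BP_attaker AI alive at its location, replacing it as each one dies.
; Tick polls the current attacker, spawns a new one when it is dead or invalid, and counts each spawn in Targe.
; The spawner destroys itself when an attacker is dead at a count of three, but an invalid reference respawns without checking the count.
; BeginPlay caches the EcoA76 player, which is otherwise unused.
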(event Custom|C_spawnAttacker
  (bind _returnvalue (AI|SpawnAIFromClass "/Game/Dragon/Attacker/BP_attaker.BP_attaker_C" 0 (Transformation|GetActorLocation) "0, 0, 0" false 0))
  (bind _asbp_attaker (Utilities|Casting|CastToBP_attaker _returnvalue))
  (Variables|Default|SetAs%20BP%20Attaker _asbp_attaker)
  (Variables|Default|Settarge (+ (Variables|Default|Gettarge) 1)))

(event EventTick
  (params (DeltaSeconds :type Float%20%28single-precision%29))
  (bind _as_bp_attaker (Variables|Default|GetAs%20BP%20Attaker))
  (Utilities|IsValid _as_bp_attaker
    (:Is%20Valid
      (if (Variables|/Game/Dragon/Attacker/BP_attaker.BP_attaker_C|GetisDead _as_bp_attaker)
        (if (== (Variables|Default|Gettarge) 3)
          (Actor|DestroyActor)
          (else
            (CallFunction|CSpawnAttacker)))))
    (:Is%20Not%20Valid
      (CallFunction|CSpawnAttacker))))

(event EventBeginPlay
  (bind _aseco_a76 (Utilities|Casting|CastToEcoA76 (Game|GetPlayerCharacter 0)))
  (Variables|Default|SetPlayer _aseco_a76))

(fn ConstructionScript)