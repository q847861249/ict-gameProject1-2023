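; AC_bullte2 is an arrow ammo pickup actor, collected with the IA_PickUP input action.
; When a Player-tagged actor overlaps its Box, it caches the first BP_flydragon and, only if that dragon's ArrowNumber is not above zero, enables input and opens a Gate.
; The input then passes the Gate, increments the dragon's ArrowNumber and destroys the pickup.
; No end-overlap logic closes the Gate or disables input.
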(event OnComponentBeginOverlap(Box)
  (params (OverlappedComponent :type Primitive%20Component%20Object%20Reference) (OtherActor :type Actor%20Object%20Reference) (OtherComp :type Primitive%20Component%20Object%20Reference) (OtherBodyIndex :type Integer) (bFromSweep :type Boolean) (SweepResult :type Hit%20Result%20Structure%20%28by%20ref%29))
  (if (Actor|ActorHasTag OtherActor "Player")
    (bind _outactors (Actor|GetAllActorsOfClass "/Game/Dragon/BP_flydragon.BP_flydragon_C"))
    (bind _output_get (Variables|Default|SetNewVar_1 (Utilities|Array|Get(acopy) _outactors)))
    (if (not (> (Variables|/Game/Dragon/BP_flydragon.BP_flydragon_C|GetarrowNumber _output_get) 0))
      (Input|EnableInput (Game|GetPlayerController 0))
      (Utilities|FlowControl|Gate true) ; enters at Open
    )))

(event Input|EnhancedActionEvents|EnhancedInputActionIA_PickUP
  (params (ActionValue :type Boolean) (ElapsedSeconds :type Float%20%28double-precision%29) (TriggeredSeconds :type Float%20%28double-precision%29) (InputAction :type Input%20Action%20Object%20Reference :default "/Game/input/Action/IA_PickUP.IA_PickUP"))
  (:Triggered
    (Utilities|FlowControl|Gate true
      (:Exit
        (Variables|/Game/Dragon/BP_flydragon.BP_flydragon_C|SetarrowNumber (stale OnComponentBeginOverlap(Box) _output_get) (+ (Variables|/Game/Dragon/BP_flydragon.BP_flydragon_C|GetarrowNumber (stale OnComponentBeginOverlap(Box) _output_get)) 1))
        (Actor|DestroyActor)))))

(event EventBeginPlay)

(event Collision|EventActorBeginOverlap
  (params (OtherActor :type Actor%20Object%20Reference)))

(event EventTick
  (params (DeltaSeconds :type Float%20%28single-precision%29)))

(fn ConstructionScript)