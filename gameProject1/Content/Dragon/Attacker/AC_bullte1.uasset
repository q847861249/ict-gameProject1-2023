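; Interactable attacker actor that lets the player spend an arrow to damage the flying dragon.
; Box overlap by a Player-tagged actor caches the first BP_flydragon and, if its ArrowNumber is positive, enables input and opens a gate.
; IA_PickUP then fires once, decrementing ArrowNumber, cutting 100 from the dragon's health struct, spawning an explosion and destroying itself.
; Leaving the box disables input but leaves the gate open.
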(event OnComponentBeginOverlap(Box)
  (params (OverlappedComponent :type Primitive%20Component%20Object%20Reference) (OtherActor :type Actor%20Object%20Reference) (OtherComp :type Primitive%20Component%20Object%20Reference) (OtherBodyIndex :type Integer) (bFromSweep :type Boolean) (SweepResult :type Hit%20Result%20Structure%20%28by%20ref%29))
  (bind _staticmesh (Variables|Default|GetStaticMesh))
  (bind _returnvalue (Transformation|GetWorldTransform _staticmesh))
  (if (Actor|ActorHasTag OtherActor "Player")
    (bind _outactors (Actor|GetAllActorsOfClass "/Game/Dragon/BP_flydragon.BP_flydragon_C"))
    (bind _output_get (Variables|Default|SetNewVar_1 (Utilities|Array|Get(acopy) _outactors)))
    (if (> (Variables|/Game/Dragon/BP_flydragon.BP_flydragon_C|GetarrowNumber _output_get) 0)
      (Input|EnableInput (Game|GetPlayerController 0))
      (Utilities|FlowControl|Gate true) ; enters at Open
    )))

(event OnComponentEndOverlap(Box)
  (params (OverlappedComponent :type Primitive%20Component%20Object%20Reference) (OtherActor :type Actor%20Object%20Reference) (OtherComp :type Primitive%20Component%20Object%20Reference) (OtherBodyIndex :type Integer))
  (if (Actor|ActorHasTag OtherActor "Player")
    (Input|DisableInput (Game|GetPlayerController 0))))

(event Input|EnhancedActionEvents|EnhancedInputActionIA_PickUP
  (params (ActionValue :type Boolean) (ElapsedSeconds :type Float%20%28double-precision%29) (TriggeredSeconds :type Float%20%28double-precision%29) (InputAction :type Input%20Action%20Object%20Reference :default "/Game/input/Action/IA_PickUP.IA_PickUP"))
  (bind _newvar_1 (Variables|Default|GetNewVar_1))
  (bind _staticmesh (Variables|Default|GetStaticMesh))
  (bind _returnvalue (Transformation|GetWorldTransform _staticmesh))
  (:Triggered
    (Utilities|FlowControl|Gate true
      (:Exit
        (Utilities|FlowControl|DoOnce false
          (:Completed
            (Variables|/Game/Dragon/BP_flydragon.BP_flydragon_C|SetarrowNumber (Variables|Default|GetNewVar_1) (- (Variables|/Game/Dragon/BP_flydragon.BP_flydragon_C|GetarrowNumber (stale OnComponentBeginOverlap(Box) _output_get)) 1))
            (Utilities|Struct|SetmembersinS_Dragon (Variables|/Game/Dragon/BP_flydragon.BP_flydragon_C|Getattibute _newvar_1) (- (.health (Variables|/Game/Dragon/BP_flydragon.BP_flydragon_C|Getattibute _newvar_1)) 1e+02) 1e+03)
            (Effects|SpawnEmitteratLocation "/Game/StarterContent/Particles/P_Explosion.P_Explosion" (.location _returnvalue) "0, 0, 0" (.scale _returnvalue))
            (Actor|DestroyActor)))))))

(event EventBeginPlay)

(event Collision|EventActorBeginOverlap
  (params (OtherActor :type Actor%20Object%20Reference)))

(event EventTick
  (params (DeltaSeconds :type Float%20%28single-precision%29)))

(fn ConstructionScript)