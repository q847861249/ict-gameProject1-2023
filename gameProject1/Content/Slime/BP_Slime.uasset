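; Slime creature Blueprint that handles movement speed and turning in reaction to heard noise.
; BeginPlay initializes Speed, and a speed_control event uses a timeline to lerp it.
; PawnSensing noise events switch on State and restart a second timeline in the Locomotion and Hit cases.
; That timeline's update lerps actor yaw toward a fixed zero rather than toward the noise location.
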(event OnHearNoise(PawnSensing)
  (params (Instigator :type Pawn%20Object%20Reference) (Location :type Vector%20%28by%20ref%29 :default "0, 0, 0") (Volume :type Float%20%28single-precision%29))
  ;[1 1 1] get location
  (switch Utilities|FlowControl|Switch|SwitchonE_Slime (Variables|Default|Getstate)
    (:NewEnumerator0
      (bind _speed (Timeline|时间轴_0 PlayFromStart)
        (:Update
          (Transformation|SetActorRotation (Math|Rotator|MakeRotator 0.0 0.0 (Math|Float|Lerp (.yaw (Transformation|GetActorRotation)) 0.0 _speed))))))
    (:NewEnumerator1
      (Timeline|时间轴_0 PlayFromStart))))

(event Custom|speed_control
  (params (speed :type Float%20%28double-precision%29))
  ;[1 1 1] speed control
  (bind _speed (Timeline|时间轴 PlayFromStart)
    (:Update
      (Variables|Default|Setspeed (Math|Float|Lerp (Variables|Default|Getspeed) speed _speed)))))

(event EventBeginPlay
  (Variables|Default|Setspeed 1.0))

(event Collision|EventActorBeginOverlap
  (params (OtherActor :type Actor%20Object%20Reference)))

(event EventTick
  (params (DeltaSeconds :type Float%20%28single-precision%29)))

(fn ConstructionScript)